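; BP_ShooterPlayerCharacter is a player character Blueprint that adds an aim camera shift and an intro sound.
; Pressing the Aim input moves Camera1 instantly to a forward and raised relative offset, and releasing it returns the camera to zero, with no interpolation or sweep.
; BeginPlay calls the parent, then plays the Intro sound at the actor's location.
; Tick and overlap events are disabled stubs, and the construction script only calls its parent.
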(event `InputAction|Aim`
  (params (Key :type "Key Structure"))
  (bind _camera1 (`self.Camera1`))
  (:`Pressed`
    (`SceneComponent.K2_SetRelativeLocation` _camera1 (100.0 0.0 50.0) false false))
  (:`Released`
    (`SceneComponent.K2_SetRelativeLocation` _camera1 (0.0 0.0 0.0) false false)))

(event `self.ReceiveBeginPlay`
  (`parent.ReceiveBeginPlay`)
  (`GameplayStatics.PlaySoundAtLocation` "/Game/AssetPacks/GameDevTV/VoiceOvers/Intro.Intro" (`self.K2_GetActorLocation`) (struct) 1.0 1.0 0.0 null null null))

(fn `UserConstructionScript`
  (`parent.UserConstructionScript`))